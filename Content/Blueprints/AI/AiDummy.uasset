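; AiDummy is a simple enemy test actor that chases the player and can be damaged and killed.
; Each tick it moves straight toward the player by setting its location without sweep or navigation, stopping within a minimum distance.
; Each hit event subtracts fixed damage from health, and reaching zero calls an empty health-pack drop stub, then destroys the actor.
; Debug strings print distance, movement and health.
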(event `self.ReceiveBeginPlay`
  (set `self.Health` 100.0))

(event `self.ReceiveHit`
  (params (MyComp :type "PrimitiveComponent Object Reference") (Other :type "Actor Object Reference") (OtherComp :type "PrimitiveComponent Object Reference") (bSelfMoved :type Boolean) (HitLocation :type "Vector Structure") (HitNormal :type "Vector Structure") (NormalImpulse :type "Vector Structure") (Hit :type "HitResult Structure (by ref)"))
  (`self.TakeDamage` 5.0))

(event `self.ReceiveTick`
  (params (DeltaSeconds :type "Float (single-precision)"))
  (`self.Move to Player` DeltaSeconds))

(fn `DropHealthPack`)

(fn `Kill`
  (`self.DropHealthPack`)
  (`self.K2_DestroyActor`))

(fn `Move to Player`
  (params (`Delta Time` :type "Float (double-precision)"))
  (locals (PlayerLoc :type "Vector Structure") (CurrentLoc :type "Vector Structure") (DeltaTime :type "Float (double-precision)"))
  (bind _returnvalue (`KismetMathLibrary.Normal` (- (`local.PlayerLoc`) (`local.CurrentLoc`))))
  (bind _returnvalue_2 (+ (`local.CurrentLoc`) (* _returnvalue (`self.Speed`) (`local.DeltaTime`))))
  ;[1 1 1] Set Local Variables
  (set `local.DeltaTime` `Delta Time`)
  (set `local.PlayerLoc` (`self.K2_GetActorLocation` (`GameplayStatics.GetPlayerCharacter` 0)))
  (bind _output_get (set `local.CurrentLoc` (`self.K2_GetActorLocation`)))
  (bind _returnvalue_3 (`KismetMathLibrary.Vector_Distance` _output_get (`local.PlayerLoc`)))
  ;[1 1 1] Determie if close enough to player, if not move toward them
  (`KismetSystemLibrary.PrintString` (`KismetStringLibrary.Conv_DoubleToString` _returnvalue_3) true true (struct :`G` 0.66 :`B` 1.0 :`A` 1.0) 2.0 "Distance")
  (if (not (< _returnvalue_3 (`self.MinDistanceToPlayer`)))
    ;[1 1 1] Move the AI toward the player
    (`KismetSystemLibrary.PrintString` (`KismetStringLibrary.Conv_VectorToString` _returnvalue) true true (struct :`G` 0.66 :`B` 1.0 :`A` 1.0) 2.0 "Normal")
    (`KismetSystemLibrary.PrintString` (`KismetStringLibrary.Conv_VectorToString` _returnvalue_2) true true (struct :`G` 0.66 :`B` 1.0 :`A` 1.0) 2.0 "TargetLoc")
    (`self.K2_SetActorLocation` _returnvalue_2)))

(fn `Spawn`)

(fn `TakeDamage`
  (params (Damage :type "Float (double-precision)"))
  ;[1 1 1] Take Damage
  (bind _output_get (set `self.Health` (- (`self.Health`) Damage)))
  ;[1 1 1] Kill if HP <= 0
  (if (<= _output_get 0.0)
    (set `self.Health` 0.0)
    (`KismetSystemLibrary.PrintString` "Dead")
    (`self.Kill`)
    (else
      (`KismetSystemLibrary.PrintString` (`KismetStringLibrary.Conv_DoubleToString` (`self.Health`))))))

(fn `UserConstructionScript`)