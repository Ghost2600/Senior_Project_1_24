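; BP_GravityZoneUp is a gravity zone actor that supplies a gravity direction for a player or object.
; GetGravityDirection ignores its input and returns the forward vector of the zone's Arrow component, so the arrow's orientation sets the direction.
; The event graph holds unreachable logic for assigning the zone through SetGravityZone and clearing it when it is the current GravityActor.
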(fn `GetGravityDirection`
  (params (PlayerOrObject :type "Actor Object Reference"))
  (returns (Direction :type "Vector Structure"))
  (return (`SceneComponent.GetForwardVector` (`self.Arrow`))))

(fn `UserConstructionScript`)