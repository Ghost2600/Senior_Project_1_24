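; BP_GravityZoneSide is a gravity zone that supplies one fixed gravity direction to test characters inside its box.
; Entering the box registers the zone on BP_TestCharacter through SetGravityZone.
; Leaving clears it only if this zone is still the character's GravityActor, so a newer zone is kept.
; GetGravityDirection returns the Arrow component's forward vector, ignoring the object passed in, so the arrow's orientation sets the pull.
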(event `self.Box.OnComponentBeginOverlap`
  (params (OverlappedComponent :type "PrimitiveComponent Object Reference") (OtherActor :type "Actor Object Reference") (OtherComp :type "PrimitiveComponent Object Reference") (OtherBodyIndex :type Integer) (bFromSweep :type Boolean) (SweepResult :type "HitResult Structure (by ref)"))
  (bind _asbp_test_character (cast `/Game/ThirdPerson/Blueprints/BP_TestCharacter` OtherActor))
  (`/Game/ThirdPerson/Blueprints/BP_TestCharacter.SetGravityZone` _asbp_test_character self))

(event `self.Box.OnComponentEndOverlap`
  (params (OverlappedComponent :type "PrimitiveComponent Object Reference") (OtherActor :type "Actor Object Reference") (OtherComp :type "PrimitiveComponent Object Reference") (OtherBodyIndex :type Integer))
  (bind _asbp_test_character (cast `/Game/ThirdPerson/Blueprints/BP_TestCharacter` OtherActor))
  (if (== (`/Game/ThirdPerson/Blueprints/BP_TestCharacter.GravityActor` _asbp_test_character) self)
    (`/Game/ThirdPerson/Blueprints/BP_TestCharacter.SetGravityZone` _asbp_test_character null)))

(fn `GetGravityDirection`
  (params (PlayerOrObject :type "Actor Object Reference"))
  (returns (Direction :type "Vector Structure"))
  (return (`SceneComponent.GetForwardVector` (`self.Arrow`))))

(fn `UserConstructionScript`)